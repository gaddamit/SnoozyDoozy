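; BP_Rotating_Ghost_Trapper is an actor that moves and rotates when activated and traps enemies that touch it.
; Activate uses MoveComponentTo on the root, offsetting its location by TargetLocation over Time, toward an absolute 90-degree rotation around the TargetRotation axis.
; Overlaps on Collision cast to BP_Enemy and call EnemyTrapped with the collision's world location.
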(event OnComponentBeginOverlap(Collision)
  (params (OverlappedComponent :type Primitive%20Component%20Object%20Reference) (OtherActor :type Actor%20Object%20Reference) (OtherComp :type Primitive%20Component%20Object%20Reference) (OtherBodyIndex :type Integer) (bFromSweep :type Boolean) (SweepResult :type Hit%20Result%20Structure%20%28by%20ref%29))
  (bind _asbp_enemy (Utilities|Casting|CastToBP_Enemy OtherActor))
  (Default|EnemyTrapped _asbp_enemy (Transformation|GetWorldLocation (Variables|Default|GetCollision))))

(event EventBeginPlay
  (|CallParentFunction) ; This node is disabled and will not be called.\nDrag off pins to build functionality.
)

(event Collision|EventActorBeginOverlap
  (params (OtherActor :type Actor%20Object%20Reference))
  (|CallParentFunction OtherActor) ; This node is disabled and will not be called.\nDrag off pins to build functionality.
)

(event EventTick
  (params (DeltaSeconds :type Float%20%28single-precision%29))
  (|CallParentFunction DeltaSeconds) ; This node is disabled and will not be called.\nDrag off pins to build functionality.
)

(event EventActivate
  (Components|MoveComponentTo (Variables|Default|GetDefaultSceneRoot) (+ (Transformation|GetWorldLocation (Variables|Default|GetDefaultSceneRoot)) (Variables|Default|GetTargetLocation)) (Math|Vector|RotatorfromAxisandAngle (Variables|Default|GetTargetRotation) 9e+01) false false (Variables|Default|GetTime) false))

(fn ConstructionScript
  (|CallParentFunction))