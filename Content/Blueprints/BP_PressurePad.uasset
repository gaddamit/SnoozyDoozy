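; Color-coded puzzle pad that opens linked doors when a BP_ColoredBlock of matching color, within a tolerance, overlaps it.
; A press sets IsPressed, waits a delay, opens each door (BP_DoorRight has its own event), then plays an optional level sequence.
; With player cheats enabled, non-block actors also trigger it.
; Construction script tints the pad; a block leaving resets only the pressed flag, if IsUnpressable.
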(event OnComponentBeginOverlap(Collision)
  (params (OverlappedComponent :type Primitive%20Component%20Object%20Reference) (OtherActor :type Actor%20Object%20Reference) (OtherComp :type Primitive%20Component%20Object%20Reference) (OtherBodyIndex :type Integer) (bFromSweep :type Boolean) (SweepResult :type Hit%20Result%20Structure%20%28by%20ref%29))
  (bind _levelsequence (Variables|Default|GetLevelSequence))
  (|IfNotPressed
    (:else
      (bind _asbp_colored_block (Utilities|Casting|CastToBP_ColoredBlock OtherActor)
        (:then
          (bind _returnvalue (CallFunction|IsSameColor _asbp_colored_block))
          (if _returnvalue
            (Variables|States|SetIsPressed true :!label _label)
            (Utilities|FlowControl|Delay (Variables|Door|GetOpenDoorDelay))
            (|OpenLinkedDoors
              (:Done
                (Utilities|IsValid _levelsequence
                  (:Is%20Valid
                    (Sequencer|Player|Play (Variables|/Script/LevelSequence.LevelSequenceActor|GetSequencePlayer _levelsequence) :!class /Script/MovieScene.MovieSceneSequencePlayer)))))))
        (:CastFailed
          (bind _asbp_player_character (Utilities|Casting|CastToBP_PlayerCharacter (Game|GetPlayerCharacter 0))) ; Check if cheats are enabled for player
          (if (Variables|/Game/Blueprints/BP_PlayerCharacter.BP_PlayerCharacter_C|GetEnableCheats _asbp_player_character)
            (goto _label)))))))

(event OnComponentEndOverlap(Collision)
  (params (OverlappedComponent :type Primitive%20Component%20Object%20Reference) (OtherActor :type Actor%20Object%20Reference) (OtherComp :type Primitive%20Component%20Object%20Reference) (OtherBodyIndex :type Integer))
  (Utilities|Casting|CastToBP_ColoredBlock OtherActor)
  (if (Variables|States|GetIsUnpressable)
    (Variables|States|SetIsPressed false)))

(fn ConstructionScript
  (bind _returnvalue (Rendering|Material|CreateDynamicMaterialInstance (Variables|Default|GetPressurePad) 0 "/Game/CuteSpace/Materials/Controllers_01_Mat.Controllers_01_Mat" "None" :!class /Script/Engine.PrimitiveComponent))
  (Rendering|Material|SetVectorParameterValue _returnvalue "PadColor" (Math|Conversions|ToLinearColor(Color) (Variables|ColorSettings|GetColor)) :!class /Script/Engine.MaterialInstanceDynamic))

(fn IsSameColor
  (params (CarryableItem :type BP%20Carryable%20Item%20Object%20Reference))
  (return (Class|KismetMathLibrary|LinearColorIsNearEqual (Math|Conversions|ToLinearColor(Color) (Variables|/Game/Blueprints/BP_CarryableItem.BP_CarryableItem_C|GetColor CarryableItem)) (Math|Conversions|ToLinearColor(Color) (Variables|ColorSettings|GetColor)) (Variables|ColorSettings|GetColorErrorTolerance))))