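; BP_Damager is an actor that damages Abe when a pressure pad activates it while Abe's color matches the pad's.
; On BeginPlay it finds the first BP_Abe in the level and caches it.
; Its Activate event compares Abe's current color name to the triggering pad's color name and calls TakeDamage on Abe when they are equal.
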(event Collision|EventActorBeginOverlap
  (params (OtherActor :type Actor%20Object%20Reference))
  (|CallParentFunction OtherActor) ; This node is disabled and will not be called.\nDrag off pins to build functionality.
)

(event EventTick
  (params (DeltaSeconds :type Float%20%28single-precision%29))
  (|CallParentFunction DeltaSeconds) ; This node is disabled and will not be called.\nDrag off pins to build functionality.
)

(event EventActivate
  (params (PressurePad :type BP%20Pressure%20Pad%20Object%20Reference))
  (bind _colorname (Default|GetCurrentColorName (Variables|Default|GetAbe)))
  (if (Utilities|Enum|Equal(Enum) _colorname (Variables|/Game/Blueprints/BP_PressurePad.BP_PressurePad_C|GetColorName PressurePad))
    (Default|TakeDamage (Variables|Default|GetAbe))))

(event EventBeginPlay
  (bind _outactors (Actor|GetAllActorsOfClass "/Game/Blueprints/BP_Abe.BP_Abe_C"))
  (bind _asbp_abe (Utilities|Casting|CastToBP_Abe (Utilities|Array|Get(acopy) _outactors)))
  (Variables|Default|SetAbe _asbp_abe))

(fn ConstructionScript
  (|CallParentFunction))