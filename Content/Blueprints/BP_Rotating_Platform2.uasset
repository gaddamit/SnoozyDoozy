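; Platform Blueprint that moves and rotates once each time its Activate event is called.
; Activate runs MoveComponentTo on the root over Time, offsetting it from its current world location by TargetLocation.
; TargetRotation is a direction vector, converted with RotationFromXVector and combined with the current relative rotation.
; The construction script only calls the parent.
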(event EventActivate
  (Components|MoveComponentTo (Variables|Default|GetDefaultSceneRoot) (+ (Transformation|GetWorldLocation (Variables|Default|GetDefaultSceneRoot)) (Variables|Default|GetTargetLocation)) (Math|Rotator|CombineRotators (Variables|/Script/Engine.SceneComponent|GetRelativeRotation (Variables|Default|GetDefaultSceneRoot)) (Math|Conversions|RotationFromXVector (Variables|Default|GetTargetRotation))) false false (Variables|Default|GetTime) false))

(fn ConstructionScript
  (|CallParentFunction))