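; BP_Abe is a boss that starts battle when the player overlaps it and summons stone monsters up to a limit.
; A state enum drives casting, summoning, damage and death.
; Tick checks whether all summons are trapped, then triggers cast-down; StartRefresh destroys them and resets the ghost trappers.
; Refreshes and damage advance a color index on the glowing stage, whose final color leads to death after damage.
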(event OnComponentBeginOverlap(DetectCollision)
  (params (OverlappedComponent :type Primitive%20Component%20Object%20Reference) (OtherActor :type Actor%20Object%20Reference) (OtherComp :type Primitive%20Component%20Object%20Reference) (OtherBodyIndex :type Integer) (bFromSweep :type Boolean) (SweepResult :type Hit%20Result%20Structure%20%28by%20ref%29))
  (Utilities|Casting|CastToBP_PlayerCharacter OtherActor)
  (if (not (Variables|Default|GetIsBattleStarted))
    (Variables|Default|SetIsBattleStarted true)
    (Variables|Default|SetStates "NewEnumerator1")))

(event Custom|Summon%20CreatureEvent
  (CallFunction|SummonCreature)
  (Math|Integer|IncrementInt (Variables|Default|GetCurrent%20Summon)))

(event Custom|Handle%20State
  (switch Utilities|FlowControl|Switch|SwitchonE_AnimationState (Variables|Default|GetStates)
    (:NewEnumerator1
      (bind _value (CallFunction|CanSummon))
      (if _value
        (Variables|Default|SetStates "NewEnumerator2")))
    (:NewEnumerator2
      (bind _value_2 (CallFunction|CanSummon))
      (if _value_2
        (Variables|Default|SetStates "NewEnumerator1")
        (else
          (Variables|Default|SetStates "NewEnumerator0"))))
    (:NewEnumerator4
      (Variables|Default|SetStates "NewEnumerator1"))
    (:NewEnumerator5
      (if (== (Variables|Default|GetCurrentColorIndex) 6)
        (Variables|Default|SetStates "NewEnumerator6")
        (else
          (Variables|Default|SetStates "NewEnumerator1"))))))

(event Custom|StartRefresh
  (CallFunction|RefreshStage)
  (Variables|Default|SetIsRefreshing false)
  (Math|Integer|IncrementInt (Variables|Default|GetCurrentColorIndex)
    (:%20%20
      (Default|ChangeMaterial (Variables|Default|GetGlowingBlocks) (Utilities|Array|Get(acopy) (Variables|Default|GetMaterialChange) (Variables|Default|GetCurrentColorIndex))))))

(event EventBeginPlay
  (|CallParentFunction)
  (Variables|Default|SetIsIdle true)
  (bind _outactors (Actor|GetAllActorsOfClass "/Game/Blueprints/BP_Ghost_Trapper.BP_Ghost_Trapper_C"))
  (Variables|Default|SetGhostTrapper _outactors)
  (bind _outactors_2 (Actor|GetAllActorsOfClass "/Game/Blueprints/BP_Glowing_Stage.BP_Glowing_Stage_C"))
  (Variables|Default|SetGlowingBlocks (Utilities|Array|Get(acopy) _outactors_2)))

(event EventTick
  (params (DeltaSeconds :type Float%20%28single-precision%29))
  (Utilities|FlowControl|Delay 1.0)
  (if (not (Variables|Default|GetIsRefreshing))
    (if (== (Variables|Default|GetCurrent%20Summon) (Variables|Default|GetMaxSummon))
      (bind _value (CallFunction|CheckAllSummonsAreTrapped))
      (if _value
        (Variables|Default|SetIsRefreshing true)
        (Variables|Default|SetStates "NewEnumerator4")))))

(fn ConstructionScript
  (|CallParentFunction))

(fn SummonCreature
  (bind _returnvalue (Game|SpawnActorfromClass "/Game/Blueprints/BP_Stone_Monster.BP_Stone_Monster_C" (Math|Transform|MakeTransform "1790.000000,-150.000000,1200.000000" "0.000000,180.000000,0.000000" "1.000000,1.000000,1.000000") "Undefined" "MultiplyWithRoot" 0 0))
  (Utilities|Array|AddUnique (Variables|Default|GetSummonedEnemies) _returnvalue)
  (Components|Sphere|SetSphereRadius (Variables|/Game/Blueprints/BP_Enemy.BP_Enemy_C|GetDetectCollision _returnvalue) 3e+03 true)
  (Variables|/Game/Blueprints/BP_Enemy.BP_Enemy_C|SetInterp%20Speed%20Position _returnvalue 0.5)
  (Variables|/Game/Blueprints/BP_Enemy.BP_Enemy_C|SetInterp%20Speed%20Rotation _returnvalue 1.0)
  (return))

(fn TrySummoning
  (if (< (Variables|Default|GetCurrent%20Summon) (Variables|Default|GetMaxSummon))
    (Variables|Default|SetStates "NewEnumerator2")))

(fn RefreshStage
  (for _array_element (Variables|Default|GetSummonedEnemies)
    (Actor|DestroyActor _array_element))
  (Utilities|Array|Clear (Variables|Default|GetSummonedEnemies))
  (for _array_element_2 (Variables|Default|GetGhostTrapper)
    (Variables|/Game/Blueprints/BP_Ghost_Trapper.BP_Ghost_Trapper_C|SetHasTrapped _array_element_2 false))
  (Variables|Default|SetCurrent%20Summon 0)
  (return))

(fn CheckAllSummonsAreTrapped
  (bind _array_element (Utilities|Array|ForEachLoopwithBreak (Variables|Default|GetSummonedEnemies) :!label _label)
    (:LoopBody
      (if (not (Variables|/Game/Blueprints/BP_Enemy.BP_Enemy_C|GetIsTrapped _array_element))
        (LocalVariables|SetAreAllSummonsTrapped false)
        (goto _label Break)))
    (:Completed
      (return (LocalVariables|GetAreAllSummonsTrapped)))))

(fn CanSummon
  (return (< (Variables|Default|GetCurrent%20Summon) (Variables|Default|GetMaxSummon))))

(fn TakeDamage
  (Variables|Default|SetStates "NewEnumerator5")
  (Math|Integer|IncrementInt (Variables|Default|GetCurrentColorIndex)
    (:%20%20
      (Default|ChangeMaterial (Variables|Default|GetGlowingBlocks) (Utilities|Array|Get(acopy) (Variables|Default|GetMaterialChange) (Variables|Default|GetCurrentColorIndex))))))

(fn GetCurrentColorName
  (return (Utilities|Array|Get(acopy) (Variables|Default|GetColorStrings) (Variables|Default|GetCurrentColorIndex))))