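; BP_Rotating_Platform is a platform actor that moves and turns when its Activate event fires.
; MoveComponentTo animates the root component over Time, offsetting its current world location by TargetLocation and adding a fixed 90-degree rotation to its relative rotation.
; Each activation computes its target from the current transform, and the construction script only calls its parent.
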(event EventActivate
  (Components|MoveComponentTo (Variables|Default|GetDefaultSceneRoot) (+ (Transformation|GetWorldLocation (Variables|Default|GetDefaultSceneRoot)) (Variables|Default|GetTargetLocation)) (Math|Rotator|CombineRotators (Variables|/Script/Engine.SceneComponent|GetRelativeRotation (Variables|Default|GetDefaultSceneRoot)) "0.000000,0.000000,90.000000") false false (Variables|Default|GetTime) false))

(fn ConstructionScript
  (|CallParentFunction))