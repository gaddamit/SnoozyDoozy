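; BP_Door_Base is a door Blueprint that swings open around a hinge component when activated.
; Its Activate event checks and sets an IsActivated flag so it fires only once, with no logic to close or reset the door.
; A Timeline then drives the Hinge's relative yaw through its DoorRotation track, without sweep.
; Tick, overlap and BeginPlay are unused, and NewFunction is an empty stub.
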(event EventBeginPlay)

(event Collision|EventActorBeginOverlap
  (params (OtherActor :type Actor%20Object%20Reference))
  (|CallParentFunction OtherActor) ; This node is disabled and will not be called.\nDrag off pins to build functionality.
)

(event EventTick
  (params (DeltaSeconds :type Float%20%28single-precision%29))
  (|CallParentFunction DeltaSeconds) ; This node is disabled and will not be called.\nDrag off pins to build functionality.
)

(event EventActivate
  (if (not (Variables|Default|GetIsActivated))
    (Variables|Default|SetIsActivated true)
    (bind _doorrotation (Timeline|Timeline Play)
      (:Update
        (Transformation|SetRelativeRotation (Variables|Default|GetHinge) (Math|Rotator|MakeRotator 0.0 0.0 _doorrotation) false false)))))

(fn ConstructionScript
  (|CallParentFunction))

(fn NewFunction)