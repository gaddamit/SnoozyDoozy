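; BP_Enemy is an enemy actor that homes in on the player character once detected and can be immobilized by a trap.
; The construction script sizes the DetectCollision sphere from DetectRange, and player overlap permanently flags the target in range.
; Tick interpolates position and look-at rotation toward the first player found at BeginPlay.
; EnemyTrapped snaps it to the trap position, leaving it only turning toward a detected player.
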(event OnComponentBeginOverlap(DetectCollision)
  (params (OverlappedComponent :type Primitive%20Component%20Object%20Reference) (OtherActor :type Actor%20Object%20Reference) (OtherComp :type Primitive%20Component%20Object%20Reference) (OtherBodyIndex :type Integer) (bFromSweep :type Boolean) (SweepResult :type Hit%20Result%20Structure%20%28by%20ref%29))
  (Utilities|Casting|CastToBP_PlayerCharacter OtherActor)
  (Variables|Default|SetIsChasing true)
  (Variables|Default|SetIsTargetInRange true))

(event Custom|EnemyTrapped
  (params (TrapPosition :type Vector))
  (Transformation|SetActorLocation TrapPosition false false)
  (Variables|Default|SetIsTrapped true)
  (Variables|Default|SetIsChasing false)
  (Variables|Default|SetIsAttacking false))

(event EventBeginPlay
  (bind _outactors (Actor|GetAllActorsOfClass "/Game/Blueprints/BP_PlayerCharacter.BP_PlayerCharacter_C"))
  (Variables|Default|SetTarget (Utilities|Array|Get(acopy) _outactors)))

(event Collision|EventActorBeginOverlap
  (params (OtherActor :type Actor%20Object%20Reference)))

(event EventTick
  (params (DeltaSeconds :type Float%20%28single-precision%29))
  (bind _returnvalue (Transformation|GetActorRotation))
  (bind _returnvalue_2 (Transformation|GetActorLocation))
  (bind _target (Variables|Default|GetTarget))
  (bind _interp_speed_rotation (Variables|Default|GetInterp%20Speed%20Rotation))
  (bind _returnvalue_3 (Transformation|GetActorLocation _target))
  (bind _returnvalue_4 (Math|Rotator|FindLookatRotation _returnvalue_2 _returnvalue_3))
  (bind _returnvalue_5 (Math|Interpolation|RInterpTo _returnvalue _returnvalue_4 DeltaSeconds _interp_speed_rotation))
  (Utilities|IsValid (Variables|Default|GetTarget)
    (:Is%20Valid
      (if (and (Variables|Default|GetIsTargetInRange) (not (Variables|Default|GetIsTrapped)))
        (Transformation|SetActorLocationAndRotation (.location (Class|KismetMathLibrary|TInterpto (Math|Conversions|ToTransform(Vector) (Transformation|GetActorLocation)) (Math|Conversions|ToTransform(Vector) (Transformation|GetActorLocation (Variables|Default|GetTarget))) DeltaSeconds (Variables|Default|GetInterp%20Speed%20Position))) _returnvalue_5)
        (elif (Variables|Default|GetIsTargetInRange)
          (Transformation|SetActorRotation _returnvalue_5))))))

(fn ConstructionScript
  (Components|Sphere|SetSphereRadius (Variables|Default|GetDetectCollision) (Variables|Default|GetDetectRange) true))

(fn TrapMonster)